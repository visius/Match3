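; BP_Cell is a Match-3 board cell actor that places and displays itself from its index and ID.
; Its CellSet event converts the index to a location with GetLocationByIndex, using hardcoded grid width, spacing and offsets.
; It then writes index and ID to text components and creates a dynamic material whose Color scalar depends on whether the ID is positive.
; A lookup of the game mode's FieldWidth is present but unused.
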(event Custom|CellSet
  (bind _cellindex (Variables|Default|GetCellIndex))
  (bind (_verticallocation _horizontallication) (CallFunction|GetLocationbyIndex _cellindex 11 75))
  (Transformation|SetActorLocation (Math|Vector|MakeVector (- _verticallocation 125.0) (+ _horizontallication 1.14e+03) 125.0) false false)
  (Rendering|Components|TextRender|SetText (Variables|Default|GetCellIndexText) (Utilities|Text|ToText(Integer) (Variables|Default|GetCellIndex)))
  (Rendering|Components|TextRender|SetText (Variables|Default|GetCellIDText) (Utilities|Text|ToText(Integer) (Variables|Default|GetCellID)))
  (bind _returnvalue (Rendering|Material|CreateDynamicMaterialInstance (Variables|Default|GetPlane) 0 "/Game/Match3/Assets/CellMaterial.CellMaterial" "None" :!class /Script/Engine.PrimitiveComponent))
  (if (<= (Variables|Default|GetCellID) 0)
    (Rendering|Material|SetScalarParameterValue _returnvalue "Color" 0.0 :!class /Script/Engine.MaterialInstanceDynamic)
    (else
      (Rendering|Material|SetScalarParameterValue _returnvalue "Color" 0.1 :!class /Script/Engine.MaterialInstanceDynamic))))

(fn ConstructionScript)