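; Match-3 board chip actor with an ID-based color, debug-style text for ID and board number, and glow states.
; Dynamic materials drive color and glow, while timelines animate spawn scaling, dropping and destruction with delays based on chip number.
; Touch lifts the chip and passes its number and location to the game mode's GameLogic.
; On destruction it increments GameLogic's DelCounter and calls DropEvent.
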(event OnInputTouchBegin(SM_Cube_02)
  (params (FingerIndex :type ETouchIndex%20Enum :default "Touch1") (TouchedComponent :type Primitive%20Component%20Object%20Reference))
  (bind _returnvalue (Game|GetGameMode))
  (bind _returnvalue_2 (Transformation|GetActorLocation))
  (bind _asdas_match_3_game_mode (Utilities|Casting|CastToDAS_Match3_GameMode _returnvalue))
  (bind _gamelogic (Variables|/Game/Match3/BluePrints/DAS_Match3_GameMode.DAS_Match3_GameMode_C|GetGameLogic _asdas_match_3_game_mode))
  (Transformation|SetActorLocation (Math|Vector|MakeVector (.x _returnvalue_2) (.y _returnvalue_2) 1.7e+02) false false)
  (Variables|/Game/Match3/BluePrints/BP_GameLogic.BP_GameLogic_C|SetTouchChepNumber _gamelogic (Variables|Default|GetChipNumber))
  (Variables|/Game/Match3/BluePrints/BP_GameLogic.BP_GameLogic_C|SetTouchChepLocation _gamelogic (Variables|Default|GetChipLocation)))

(event OnInputTouchEnd(SM_Cube_02)
  (params (FingerIndex :type ETouchIndex%20Enum :default "Touch1") (TouchedComponent :type Primitive%20Component%20Object%20Reference))
  (bind _returnvalue (Transformation|GetActorLocation))
  (Transformation|SetActorLocation (Math|Vector|MakeVector (.x _returnvalue) (.y _returnvalue) 7e+01) false false))

(event Custom|EventDarkColor
  (Rendering|Material|SetScalarParameterValue (Variables|Default|GetChipMaterial) "GlowPower" 0.1 :!class /Script/Engine.MaterialInstanceDynamic))

(event Custom|ChipSpawnEwent
  (bind _id (Variables|Default|GetID))
  (Variables|Default|SetChipLocation (Transformation|GetActorLocation))
  (Rendering|Components|TextRender|SetText (Variables|Default|GetID_Chip) (Utilities|Text|ToText(Integer) _id))
  (Rendering|Components|TextRender|SetText (Variables|Default|GetChip_Numder) (Utilities|Text|ToText(Integer) (Variables|Default|GetChipNumber)))
  (switch int _id
    (:1
      (Variables|Default|SetColor (Variables|ChipColors|GetPink)))
    (:2
      (Variables|Default|SetColor (Variables|ChipColors|GetRed)))
    (:3
      (Variables|Default|SetColor (Variables|ChipColors|GetYelow)))
    (:4
      (Variables|Default|SetColor (Variables|ChipColors|GetBlue)))
    (:5
      (Variables|Default|SetColor (Variables|ChipColors|GetGreen))))
  (Utilities|FlowControl|Sequence
    (:then_0
      (bind _returnvalue (Rendering|Material|CreateDynamicMaterialInstance (Variables|Default|GetSM_Cube_02) 0 "/Game/Match3/Assets/M_Cheps_01.M_Cheps_01" "None" :!class /Script/Engine.PrimitiveComponent))
      (Variables|Default|SetChipMaterial _returnvalue)
      (Rendering|Material|SetVectorParameterValue _returnvalue "TrimColor" (Variables|Default|GetColor) :!class /Script/Engine.MaterialInstanceDynamic)
      (Rendering|Material|SetVectorParameterValue _returnvalue "FloorColor" (Variables|Default|GetColor) :!class /Script/Engine.MaterialInstanceDynamic)
      (Rendering|Material|SetVectorParameterValue _returnvalue "GlowColor" (Variables|Default|GetColor) :!class /Script/Engine.MaterialInstanceDynamic)
      (Rendering|Material|SetScalarParameterValue _returnvalue "GlowPower" (Variables|Default|GetGlowPower) :!class /Script/Engine.MaterialInstanceDynamic))
    (:then_1
      (bind _returnvalue_2 (Rendering|Material|CreateDynamicMaterialInstance (Variables|Default|GetID_Chip) 0 "/Game/Match3/Assets/DefaultTextMaterialOpaque.DefaultTextMaterialOpaque" "None" :!class /Script/Engine.PrimitiveComponent))
      (Rendering|Material|SetVectorParameterValue _returnvalue_2 "TextColor" (/ (Variables|Default|GetColor) (Math|Conversions|ToLinearColor(Float) (Variables|Default|GetTextColorDevider))) :!class /Script/Engine.MaterialInstanceDynamic)
      (bind _returnvalue_3 (Rendering|Material|CreateDynamicMaterialInstance (Variables|Default|GetChip_Numder) 0 "/Game/Match3/Assets/DefaultTextMaterialOpaque.DefaultTextMaterialOpaque" "None" :!class /Script/Engine.PrimitiveComponent))
      (Rendering|Material|SetVectorParameterValue _returnvalue_3 "TextColor" (/ (Variables|Default|GetColor) (Math|Conversions|ToLinearColor(Float) 3.0)) :!class /Script/Engine.MaterialInstanceDynamic)
      (Transformation|SetActorScale3D "0, 0, 0"))
    (:then_2
      ;[1 1 1] AnimateSpawn
      (Utilities|FlowControl|Delay (/ (* (Math|Random|RandomFloatinRange 0.0 0.15) (Math|Conversions|ToFloat(Integer) (Variables|Default|GetChipNumber))) 4e+01))
      (bind _scale (Timeline|Timeline_1 Play)
        (:Update
          (Transformation|SetActorScale3D (Math|Conversions|ToVector(Float) _scale)))))))

(event Custom|BorderColor
  (bind _chipmaterial (Variables|Default|GetChipMaterial))
  (Rendering|Material|SetScalarParameterValue _chipmaterial "BorderGlow" 1e+02 :!class /Script/Engine.MaterialInstanceDynamic)
  (Rendering|Material|SetScalarParameterValue _chipmaterial "GlowPower" 0.1 :!class /Script/Engine.MaterialInstanceDynamic))

(event Custom|ChangeColor
  (bind _chipmaterial (Variables|Default|GetChipMaterial))
  (bind _chipmaterial_2 (Variables|Default|GetChipMaterial))
  (switch int (Variables|Default|GetID)
    (:1
      (Variables|Default|SetColor (Variables|ChipColors|GetPink)))
    (:2
      (Variables|Default|SetColor (Variables|ChipColors|GetRed)))
    (:3
      (Variables|Default|SetColor (Variables|ChipColors|GetYelow)))
    (:4
      (Variables|Default|SetColor (Variables|ChipColors|GetBlue)))
    (:5
      (Variables|Default|SetColor (Variables|ChipColors|GetGreen))))
  (Rendering|Material|SetVectorParameterValue _chipmaterial_2 "TrimColor" (Variables|Default|GetColor) :!class /Script/Engine.MaterialInstanceDynamic)
  (Rendering|Material|SetVectorParameterValue _chipmaterial_2 "FloorColor" (Variables|Default|GetColor) :!class /Script/Engine.MaterialInstanceDynamic)
  (Rendering|Material|SetVectorParameterValue _chipmaterial_2 "GlowColor" (Variables|Default|GetColor) :!class /Script/Engine.MaterialInstanceDynamic)
  (Rendering|Components|TextRender|SetText (Variables|Default|GetID_Chip) (Utilities|Text|ToText(Integer) (Variables|Default|GetID)))
  (Rendering|Material|SetScalarParameterValue _chipmaterial "GlowPower" 0.2 :!class /Script/Engine.MaterialInstanceDynamic)
  (Rendering|Material|SetScalarParameterValue _chipmaterial "BorderGlow" 1e+02 :!class /Script/Engine.MaterialInstanceDynamic))

(event Custom|EventResetColor
  (bind _chipmaterial (Variables|Default|GetChipMaterial))
  (Rendering|Material|SetScalarParameterValue _chipmaterial "GlowPower" 1.0 :!class /Script/Engine.MaterialInstanceDynamic)
  (Rendering|Material|SetScalarParameterValue _chipmaterial "BorderGlow" 1.0 :!class /Script/Engine.MaterialInstanceDynamic))

(event Custom|Destroy
  ;[1 0.1176 0.1094] Destroy Chip
  (Utilities|FlowControl|Delay (/ (* (Math|Random|RandomFloatinRange 0.0 0.15) (Math|Conversions|ToFloat(Integer) (Variables|Default|GetChipNumber))) 5e+01))
  (bind _scale (Timeline|Timeline_0 Play)
    (:Update
      (Transformation|SetActorScale3D (Math|Conversions|ToVector(Float) _scale)))
    (:Finished
      (Actor|DestroyActor))))

(event Custom|EventGlowEffect
  (Rendering|Material|SetScalarParameterValue (Variables|Default|GetChipMaterial) "GlowPower" 4.0 :!class /Script/Engine.MaterialInstanceDynamic))

(event Custom|ChipDrop
  (params (ChipNumber :type Integer) (ChipLocation :type Vector))
  (Utilities|FlowControl|Delay (* (/ 1.0 (Math|Conversions|ToFloat(Integer) ChipNumber)) 3.0))
  (bind _newtrack_0 (Timeline|DropTimeLine PlayFromStart)
    (:Update
      _)
    (:Finished
      (Variables|Default|SetChipLocation ChipLocation)
      (Variables|Default|SetChipNumber ChipNumber)))
  (Transformation|SetActorLocation (Math|Vector|MakeVector (.X (Math|Vector|BreakVector (Math|Vector|Lerp(Vector) (Variables|Default|GetChipLocation) ChipLocation _newtrack_0))) (.Y (Math|Vector|BreakVector (Math|Vector|Lerp(Vector) (Variables|Default|GetChipLocation) ChipLocation _newtrack_0))) (.Z (Math|Vector|BreakVector (Math|Vector|Lerp(Vector) (Variables|Default|GetChipLocation) ChipLocation _newtrack_0)))) false false)
  (Rendering|Components|TextRender|SetText (Variables|Default|GetChip_Numder) (Utilities|Text|ToText(Integer) (Variables|Default|GetChipNumber))))

(event EventDestroyed
  (bind _returnvalue (Game|GetGameMode))
  (bind _asdas_match_3_game_mode (Utilities|Casting|CastToDAS_Match3_GameMode _returnvalue))
  (bind _gamelogic (Variables|/Game/Match3/BluePrints/DAS_Match3_GameMode.DAS_Match3_GameMode_C|GetGameLogic _asdas_match_3_game_mode))
  (Math|Integer|IncrementInt (Variables|/Game/Match3/BluePrints/BP_GameLogic.BP_GameLogic_C|GetDelCounter _gamelogic)
    (:%20%20
      (Default|DropEvent _gamelogic))))

(fn ConstructionScript)

(fn ChipSet
  (params (ChipNumber :type Integer) (ChipLocation :type Vector))
  (Variables|Default|SetChipNumber ChipNumber)
  (Transformation|SetActorLocation ChipLocation false false)
  (Variables|Default|SetChipLocation ChipLocation)
  (Rendering|Components|TextRender|SetText (Variables|Default|GetChip_Numder) (Utilities|Text|ToText(Integer) (Variables|Default|GetChipNumber))))