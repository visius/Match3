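; Player controller for the Match-3 game that turns touch drags into four-way swipes and quits the game on Escape.
; Finger1 press records the start point, and Tick polls the touch until it moves past a small distance threshold.
; The dominant axis and sign set the swipe enum, which goes to GameLogic.SwipeEvent on the game mode.
; A DoOnce, reset on release, limits this to one swipe per touch.
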(event EventTick
  (params (DeltaSeconds :type Float%20%28single-precision%29))
  (bind _returnvalue (Game|GetPlayerController 0))
  (bind (_locationx _locationy) (Class|PlayerController|GetInputTouchState _returnvalue "Touch1"))
  (bind _returnvalue_2 (Math|Vector2D|MakeVector2D _locationx _locationy))
  ;[1 1 1] Swipe
  (if (Variables|Default|GetIsTouched)
    (if (> (Math|Vector2D|Vector2DLength (- (Variables|Default|GetTouchStart) _returnvalue_2)) 25.0)
      (Utilities|FlowControl|DoOnce false
        (:Completed
          (Variables|Default|SetTouchEnd _returnvalue_2)
          (if (!= (Math|Float|Absolute(Float) (.x (- (Variables|Default|GetTouchStart) (Variables|Default|GetTouchEnd)))) (Math|Float|Absolute(Float) (.y (- (Variables|Default|GetTouchStart) (Variables|Default|GetTouchEnd)))))
            (if (> (Math|Float|Absolute(Float) (.x (- (Variables|Default|GetTouchStart) (Variables|Default|GetTouchEnd)))) (Math|Float|Absolute(Float) (.y (- (Variables|Default|GetTouchStart) (Variables|Default|GetTouchEnd)))))
              (if (> (.x (- (Variables|Default|GetTouchStart) (Variables|Default|GetTouchEnd))) 0.0)
                (Variables|Default|SetSwipesEnum "NewEnumerator0")
                (else
                  (Variables|Default|SetSwipesEnum "NewEnumerator1")))
              (elif (> (.y (- (Variables|Default|GetTouchStart) (Variables|Default|GetTouchEnd))) 0.0)
                (Variables|Default|SetSwipesEnum "NewEnumerator2")
                (else
                  (Variables|Default|SetSwipesEnum "NewEnumerator3"))))
            (Default|SwipeEvent (Variables|/Game/Match3/BluePrints/DAS_Match3_GameMode.DAS_Match3_GameMode_C|GetGameLogic (.AsDAS%20Match%203%20Game%20Mode (Utilities|Casting|CastToDAS_Match3_GameMode (Game|GetGameMode)))) (Variables|Default|GetSwipesEnum))))))))

(event Input|ActionEvents|InputActionFinger1
  (params (Key :type Key%20Structure))
  (bind _returnvalue (Game|GetPlayerController 0))
  (bind (_locationx _locationy) (Class|PlayerController|GetInputTouchState _returnvalue "Touch1"))
  (bind _returnvalue_2 (Math|Vector2D|MakeVector2D _locationx _locationy))
  ;[1 1 1] Swipe
  (:Pressed
    (Variables|Default|SetIsTouched true)
    (Variables|Default|SetTouchStart _returnvalue_2))
  (:Released
    (Variables|Default|SetIsTouched false)
    (Utilities|FlowControl|DoOnce false) ; enters at Reset
  ))

(event Input|KeyboardEvents|Escape
  (params (Key :type Key%20Structure))
  ;[1 1 1] QuitGame
  (:Released
    (Development|ExecuteConsoleCommand "quit game" 0)))

(fn ConstructionScript)